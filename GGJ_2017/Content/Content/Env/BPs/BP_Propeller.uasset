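; BP_Propeller is an environment actor that reacts to the player Minotaur's FireForce event with an impulse and a round-trip move.
; The event applies an off-center upward impulse to the Propeller component and restarts the cycle.
; Tick eases the actor between its placed location and TargetB with VInterpTo, stopping after a round trip.
; HalfCycle raises interp speed and is never reset; Preview adds an arrow at TargetB.
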(event Custom|TriggerBitch
  (bind _propeller (Variables|Default|GetPropeller))
  (Variables|Default|SethasFinishedWholeCycle? false)
  (Physics|AddImpulseatLocation _propeller "0.000000, 0,50000.000000" (+ (Transformation|GetWorldLocation _propeller) "0.000000,50.000000,50.000000") "None"))

(event EventBeginPlay
  (bind _asminotaur (Utilities|Casting|CastToMinotaur (Game|Player|GetPlayerPawn 0)))
  (EventDispatchers|BindEventtoFireForce _asminotaur (delegate Custom|TriggerBitch)))

(event EventTick
  (params (DeltaSeconds :type Float%20%28single-precision%29))
  (if (not (Variables|Default|GethasFinishedWholeCycle?))
    (CallFunction|UpdateLocation)))

(fn ConstructionScript
  ;[1 1 1] Setup Target A
  (Variables|Platform|SetTargetA (Transformation|GetActorLocation))
  (Variables|Platform|SetTargetCurr (Variables|Platform|GetTargetB))
  (if (Variables|General|GetPreview)
    (AddComponent|AddArrowComponent false (Math|Transform|MakeTransform (Variables|Platform|GetTargetB) "90.000000,0.000000, 0" "2.000000,2.000000,2.000000"))))

(fn UpdateLocation
  (if (< (Math|Vector|VectorLength (- (Variables|Platform|GetTargetCurr) (Transformation|GetActorLocation))) 1e+01)
    (if (Variables|Platform|GetmovingTowardsB?)
      (Variables|Platform|SetTargetCurr (Variables|Platform|GetTargetA))
      (Variables|Platform|SetmovingTowardsB? false)
      (Variables|Default|SethalfCycle? true)
      (else
        (Variables|Platform|SetTargetCurr (Variables|Platform|GetTargetB))
        (Variables|Platform|SetmovingTowardsB? true)
        (if (Variables|Default|GethalfCycle?)
          (Variables|Default|SethasFinishedWholeCycle? true))))
    (else
      (Transformation|SetActorLocation (Math|Interpolation|VInterpTo (Transformation|GetActorLocation) (Variables|Platform|GetTargetCurr) (Utilities|Time|GetWorldDeltaSeconds) (+ (Math|Conversions|ToFloat(Boolean) (Variables|Default|GethalfCycle?)) (Variables|Platform|GetInterpSpeed))) false false))))