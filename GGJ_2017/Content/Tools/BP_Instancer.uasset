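; BP_Instancer is a tool actor that renders one mesh at many transforms through an Instanced Static Mesh component.
; Its construction script adds that component at the actor's transform, assigns InstancedMesh, then adds a world-space instance for each entry in the Transforms array.
; All work happens at construction, and BeginPlay is empty.
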(event EventBeginPlay)

(fn ConstructionScript
  (CallFunction|InitInstancer)
  (CallFunction|GatherInstances))

(fn GatherInstances
  (bind _instances (Variables|Components|GetInstances))
  ;[1 1 1] Clear the instances and supply the mesh
  (Components|InstancedStaticMesh|ClearInstances _instances)
  (Components|StaticMesh|SetStaticMesh _instances (Variables|Instancing|GetInstanced%20Mesh))
  (for _array_element (Variables|Instancing|GetTransforms)
    (Class|InstancedStaticMeshComponent|AddInstanceWorldSpace (Variables|Components|GetInstances) _array_element)))

(fn InitInstancer
  (bind _returnvalue (AddComponent|AddInstancedStaticMeshComponent false (Transformation|GetActorTransform)))
  (Variables|Components|SetInstances _returnvalue))