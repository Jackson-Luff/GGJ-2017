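; BP_Spliner is a construction-time tool that lays a chosen static mesh along its spline.
; InitSplineMesh adds a spline mesh component for each segment between consecutive points, with a configurable forward axis and query-only collision.
; Helper functions supply each segment's start and end locations and tangents to bend the mesh along the curve.
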(fn ConstructionScript
  (SplineCreation|InitSplineMesh))

(fn InitSplineMesh
  (for _index (range 0 (- (Spline|GetNumberOfSplinePoints (Variables|Default|GetSpline)) 2))
    (LocalVariables|SetIndex _index)
    (bind _returnvalue (AddComponent|AddSplineMeshComponent true))
    (Components|StaticMesh|SetStaticMesh _returnvalue (Variables|SplineCreation|GetMesh))
    (SplineMesh|SetForwardAxis _returnvalue (Variables|SplineCreation|GetMeshFwdAxis) true)
    (Transformation|AttachComponentToComponent _returnvalue (Variables|Default|GetSpline) "None" "KeepWorld" "KeepWorld" "KeepWorld" true)
    (SplineCreation|SetLocandTangatPoint (LocalVariables|GetIndex) (LocalVariables|GetStart_Loc) (LocalVariables|GetStart_Tang))
    (SplineCreation|SetLocandTangatPoint (+ (LocalVariables|GetIndex) 1) (LocalVariables|GetEnd_Loc) (LocalVariables|GetEnd_Tang))
    (SplineMesh|SetStartandEnd _returnvalue (LocalVariables|GetStart_Loc) (LocalVariables|GetStart_Tang) (LocalVariables|GetEnd_Loc) (LocalVariables|GetEnd_Tang) true :!class /Script/Engine.SplineMeshComponent)
    (Collision|SetCollisionEnabled _returnvalue "QueryOnly")))

(fn SetLocandTangatPoint
  (params (Index :type Integer) (rLocation :type Vector%20%28by%20ref%29) (rTanget :type Vector%20%28by%20ref%29))
  (bind (_location _tangent) (Utilities|GetLocandTangatPoint Index))
  (|SetBy-RefVar rLocation _location)
  (|SetBy-RefVar rTanget _tangent)
  (return))